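; BP_Drink is a pickup actor that passes an HP recovery amount to the player who touches it.
; Tick spins the Cylinder component around yaw at a constant, frame-rate-independent speed.
; When SphereCollision begins overlapping a BP_PlayerCharacter, it calls GetDrink on that character with HPRecoveryAmount, then destroys itself.
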(event OnComponentBeginOverlap(SphereCollision)
  (params (OverlappedComponent :type Primitive%20Component%20Object%20Reference) (OtherActor :type Actor%20Object%20Reference) (OtherComp :type Primitive%20Component%20Object%20Reference) (OtherBodyIndex :type Integer) (bFromSweep :type Boolean) (SweepResult :type Hit%20Result%20Structure%20%28by%20ref%29))
  (bind _asbp_player_character (Utilities|Casting|CastToBP_PlayerCharacter OtherActor))
  (Default|GetDrink _asbp_player_character (Variables|Default|GetHP%20recovery%20amount))
  (Actor|DestroyActor))

(event EventBeginPlay)

(event Collision|EventActorBeginOverlap
  (params (OtherActor :type Actor%20Object%20Reference)))

(event EventTick
  (params (DeltaSeconds :type Float%20%28single-precision%29))
  (bind _cylinder (Variables|Default|GetCylinder))
  (bind _returnvalue (Transformation|GetRelativeTransform _cylinder))
  (Transformation|SetRelativeRotation _cylinder (Math|Rotator|MakeRotator (.roll (.rotation _returnvalue)) (.pitch (.rotation _returnvalue)) (+ (.yaw (.rotation _returnvalue)) (* DeltaSeconds 1.2e+02))) false false))

(fn ConstructionScript)